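; Track tile for an endless runner that populates itself with random obstacles, boxes or coins on BeginPlay.
; SpawnObstacles rolls Lane1 first, rolling Lane0 only after an Obstacle lands there, and Lane2 only after another in Lane0.
; When the character overlaps the Box, the tile asks the game mode for another tile and adds multiplied points.
; It also raises walk speed slightly within clamped limits, then destroys itself after a delay.
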(event OnComponentBeginOverlap(Box)
  (params (OverlappedComponent :type Primitive%20Component%20Object%20Reference) (OtherActor :type Actor%20Object%20Reference) (OtherComp :type Primitive%20Component%20Object%20Reference) (OtherBodyIndex :type Integer) (bFromSweep :type Boolean) (SweepResult :type Hit%20Result%20Structure%20%28by%20ref%29))
  (Utilities|Casting|CastToThirdPersonCharacter OtherActor)
  (bind _asthird_person_game_mode (Utilities|Casting|CastToThirdPersonGameMode (Game|GetGameMode)))
  (Default|SpwanTile _asthird_person_game_mode)
  ;[1 1 1] Score
  (bind _asthird_person_game_mode_2 (Utilities|Casting|CastToThirdPersonGameMode (Game|GetGameMode)))
  (bind _output_get (Variables|/Game/ThirdPersonBP/Blueprints/ThirdPersonGameMode.ThirdPersonGameMode_C|SetCurrentPoints _asthird_person_game_mode_2 (+ (* 1 (Variables|/Game/ThirdPersonBP/Blueprints/ThirdPersonGameMode.ThirdPersonGameMode_C|GetPointsMultiplier _asthird_person_game_mode_2)) (Variables|/Game/ThirdPersonBP/Blueprints/ThirdPersonGameMode.ThirdPersonGameMode_C|GetCurrentPoints _asthird_person_game_mode_2))))
  (Development|PrintString (Utilities|String|ToString(Integer) _output_get))
  ;[1 1 1] Speed
  (bind _asthird_person_character (Utilities|Casting|CastToThirdPersonCharacter (Game|GetPlayerCharacter 0)))
  (Variables|/Script/Engine.CharacterMovementComponent|SetMaxWalkSpeed (Variables|/Script/Engine.Character|GetCharacterMovement _asthird_person_character) (Math|Float|Clamp(Float) (* (Variables|/Script/Engine.CharacterMovementComponent|GetMaxWalkSpeed (Variables|/Script/Engine.Character|GetCharacterMovement _asthird_person_character)) 1.01) 6e+02 2e+03))
  (Utilities|FlowControl|Delay 2.5)
  (Actor|DestroyActor))

(event EventBeginPlay
  (CallFunction|SpawnObstacles))

(event Collision|EventActorBeginOverlap
  (params (OtherActor :type Actor%20Object%20Reference)))

(event EventTick
  (params (DeltaSeconds :type Float%20%28single-precision%29)))

(fn ConstructionScript)

(fn SpawnObstacles
  (bind _lane1 (Variables|Default|GetLane1))
  (bind _lane0 (Variables|Default|GetLane0))
  (bind _lane2 (Variables|Default|GetLane2))
  (bind _returnvalue (Transformation|GetWorldTransform _lane2))
  (bind _returnvalue_2 (Transformation|GetWorldTransform _lane1))
  (bind _returnvalue_3 (Transformation|GetWorldTransform _lane0))
  ;[1 1 1] Lane 0
  (switch int (Math|Random|RandomIntegerinRange 0 3)
    (:1
      (Game|SpawnActorfromClass "/Game/RunnerFiles/Blueprints/Obstacle.Obstacle_C" _returnvalue_2 "Undefined" 0 0)
      ;[1 1 1] Lane 1
      (switch int (Math|Random|RandomIntegerinRange 0 3)
        (:1
          (Game|SpawnActorfromClass "/Game/RunnerFiles/Blueprints/Obstacle.Obstacle_C" _returnvalue_3 "Undefined" 0 0)
          ;[1 1 1] Lane 2
          (switch int (Math|Random|RandomIntegerinRange 0 3)
            (:1
              (Game|SpawnActorfromClass "/Game/RunnerFiles/Blueprints/Obstacle.Obstacle_C" _returnvalue "Undefined" 0 0))
            (:2
              (Game|SpawnActorfromClass "/Game/RunnerFiles/Blueprints/Obstacle_Box.Obstacle_Box_C" _returnvalue "Undefined" 0 0))
            (:3
              (Game|SpawnActorfromClass "/Game/RunnerFiles/Blueprints/Coin.Coin_C" _returnvalue "Undefined" 0 0))))
        (:2
          (Game|SpawnActorfromClass "/Game/RunnerFiles/Blueprints/Obstacle_Box.Obstacle_Box_C" _returnvalue_3 "Undefined" 0 0))
        (:3
          (Game|SpawnActorfromClass "/Game/RunnerFiles/Blueprints/Coin.Coin_C" _returnvalue_3 "Undefined" 0 0))))
    (:2
      (Game|SpawnActorfromClass "/Game/RunnerFiles/Blueprints/Obstacle_Box.Obstacle_Box_C" _returnvalue_2 "Undefined" 0 0))
    (:3
      (Game|SpawnActorfromClass "/Game/RunnerFiles/Blueprints/Coin.Coin_C" _returnvalue_2 "Undefined" 0 0))))